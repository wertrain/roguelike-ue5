(event `self.Create`
  (params (Type :type "EItemType Enum" :default "Sword"))
  (`parent.Create` Type)
  (`self.LoadMesh` Type))

(fn `LoadMesh`
  (params (ItemType :type "EItemType Enum" :default "Sword"))
  (`SceneComponent.ResetRelativeTransform` (`self.DefaultSceneRoot`))
  (switch `EItemType` ItemType
    (:`Sword`
      (`StaticMeshComponent.SetStaticMesh` (`self.StaticMesh`) "/Game/Asset/Item/SwordIron/SM_SwordIron.SM_SwordIron")
      (`SceneComponent.SetWorldScale3D` (`self.DefaultSceneRoot`) (0.5 0.2 0.5))
      (`SceneComponent.K2_AddLocalOffset` (`self.StaticMesh`) (0.0 0.0 80.0) false true))
    (:`Shield`
      (`StaticMeshComponent.SetStaticMesh` (`self.StaticMesh`) "/Game/Asset/Item/ShieldWood/SM_ShieldWood.SM_ShieldWood")
      (`SceneComponent.SetWorldScale3D` (`self.DefaultSceneRoot`) (1.0 1.0 1.0))
      (`SceneComponent.K2_AddLocalOffset` (`self.StaticMesh`) (0.0 0.0 40.0) false true))))

(fn `UserConstructionScript`
  (`self.Create` "Shield"))